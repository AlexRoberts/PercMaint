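; SpawnZone is an enemy spawn area that creates a wave of BaseEnemy actors inside its Box component on demand.
; SpawnWave takes a count, starting health and attack damage, then spawns each enemy at a random point in the box's bounds, adjusting for collisions but always spawning.
; Each enemy is owned by the player character, receives its default controller, then has its health and damage set.
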(fn `SpawnWave`
  (params (`#Enemies` :type Integer) (StartingHealth :type "Float (double-precision)") (AttackDamage :type "Float (double-precision)"))
  (bind (_origin _boxextent) (`KismetSystemLibrary.GetComponentBounds` (`self.Box`)))
  (for _ (range `#Enemies`)
    (bind _returnvalue (`|SpawnActorFromClass` "/Game/Blueprints/Enemy/BaseEnemy.BaseEnemy_C" (`KismetMathLibrary.MakeTransform` (`KismetMathLibrary.RandomPointInBoundingBox` _origin _boxextent)) "AdjustIfPossibleButAlwaysSpawn" "OverrideRootScale" (`GameplayStatics.GetPlayerCharacter` 0)))
    (`Pawn.SpawnDefaultController` _returnvalue)
    (bind _output_get (set `/Game/Blueprints/Enemy/BaseEnemy.MaxHealth` StartingHealth _returnvalue))
    (set `/Game/Blueprints/Enemy/BaseEnemy.Health` _output_get _returnvalue)
    (set `/Game/Blueprints/Enemy/BaseEnemy.AttackDamage` AttackDamage _returnvalue)))

(fn `UserConstructionScript`)