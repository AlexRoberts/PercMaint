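; Lava hazard actor that periodically damages the player while they stand inside its box volume.
; Box begin overlap caches the TopDownCharacter, and a looping one-second timer applies LavaDamage through TakeDamage while that character still overlaps.
; Enemy damage is inactive: end overlap removes BaseEnemy actors from Enemies, but the logic that adds and damages them is disconnected.
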(event `self.ReceiveBeginPlay`
  (`KismetSystemLibrary.K2_SetTimerDelegate` (delegate `DealDamage`) 1.0 true))

(event `self.Box.OnComponentBeginOverlap`
  (params (OverlappedComponent :type "PrimitiveComponent Object Reference") (OtherActor :type "Actor Object Reference") (OtherComp :type "PrimitiveComponent Object Reference") (OtherBodyIndex :type Integer) (bFromSweep :type Boolean) (SweepResult :type "HitResult Structure (by ref)"))
  (bind _astop_down_character (cast `/Game/TopDownBP/Blueprints/TopDownCharacter` OtherActor))
  (set `self.Character` _astop_down_character))

(event `self.Box.OnComponentEndOverlap`
  (params (OverlappedComponent :type "PrimitiveComponent Object Reference") (OtherActor :type "Actor Object Reference") (OtherComp :type "PrimitiveComponent Object Reference") (OtherBodyIndex :type Integer))
  (bind _asbase_enemy (cast `/Game/Blueprints/Enemy/BaseEnemy` OtherActor))
  (`KismetArrayLibrary.Array_RemoveItem` (`self.Enemies`) _asbase_enemy))

(event `DealDamage`
  (bind _character (`self.Character`))
  (`|ExecutionSequence`
    (:`then_0`
      (if (and (`PrimitiveComponent.IsOverlappingActor` (`self.Box`) _character) (`KismetSystemLibrary.IsValid` _character))
        (`/Game/TopDownBP/Blueprints/TopDownCharacter.TakeDamage` _character (`self.LavaDamage`))))))

(fn `UserConstructionScript`)