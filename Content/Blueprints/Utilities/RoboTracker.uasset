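; RoboTracker is a short-lived AI-moved pawn that travels toward a target actor, drawing a particle trail attached to its sphere.
; Its Go event receives the target and owning pawn, then starts AI Move To and two one-shot timers.
; It destroys itself when the move succeeds or fails, when a half-second check finds it too far from its owner, or after one second.
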(event `self.ReceiveBeginPlay`
  (`GameplayStatics.SpawnEmitterAttached` "/Game/FX/Trail_P.Trail_P" (`self.Sphere`) "None" (0.0 0.0 0.0) (struct) "SnapToTarget"))

(event `Go`
  (params (TargetActor :type "Actor Object Reference") (OwningPawn :type "Actor Object Reference"))
  (`|AIMoveTo` self (0.0 0.0 0.0) TargetActor
    (:`then`
      (bind _returnvalue (`KismetSystemLibrary.K2_SetTimerDelegate` (delegate `CheckDist`) 0.5))
      (`KismetSystemLibrary.K2_SetTimerDelegate` (delegate `kill`) 1.0))
    (:`OnSuccess`
      (`self.K2_DestroyActor` :!label _label)
      (`KismetSystemLibrary.K2_ClearAndInvalidateTimerHandle` _returnvalue))
    (:`OnFail`
      (goto _label))))

(event `CheckDist`
  (if (> (`self.GetDistanceTo` (stale `Go` OwningPawn)) 1000.0)
    (goto _label)))

(event `kill`
  (goto _label))

(fn `UserConstructionScript`)