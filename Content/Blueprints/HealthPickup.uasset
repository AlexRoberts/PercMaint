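; Health pickup actor that restores health to a TopDownCharacter on overlap and then destroys itself.
; A short delay after BeginPlay enables pickup, and a timer destroys the actor if it is not collected in time.
; The box overlap heals by HealthAmount, clamped to MaxHealth, and only consumes the pickup when the character is below full health.
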(event `self.ReceiveBeginPlay`
  (`KismetSystemLibrary.K2_SetTimerDelegate` (delegate `Expire`) 10.0)
  (`KismetSystemLibrary.Delay` 1.0)
  (set `self.CanPickUp` true))

(event `Expire`
  (`self.K2_DestroyActor`))

(event `self.Box.OnComponentBeginOverlap`
  (params (OverlappedComponent :type "PrimitiveComponent Object Reference") (OtherActor :type "Actor Object Reference") (OtherComp :type "PrimitiveComponent Object Reference") (OtherBodyIndex :type Integer) (bFromSweep :type Boolean) (SweepResult :type "HitResult Structure (by ref)"))
  (if (`self.CanPickUp`)
    (bind _astop_down_character (cast `/Game/TopDownBP/Blueprints/TopDownCharacter` OtherActor))
    (bind _health (`/Game/TopDownBP/Blueprints/TopDownCharacter.Health` _astop_down_character))
    (bind _maxhealth (`/Game/TopDownBP/Blueprints/TopDownCharacter.MaxHealth` _astop_down_character))
    (if (< _health _maxhealth)
      (set `/Game/TopDownBP/Blueprints/TopDownCharacter.Health` (`KismetMathLibrary.FClamp` (+ _health (`self.HealthAmount`)) 0.0 _maxhealth) _astop_down_character)
      (`self.K2_DestroyActor`))))

(fn `UserConstructionScript`)